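; BP_PrintObjectInfo_SkeletalMesh is a Blueprint that prints debug information about its skeletal mesh component.
; The PrintObjectInfo event builds one Japanese-labelled string with the mesh name, material count, material names and bone count, printing it to screen and/or log as its parameters select.
; GetMaterialStr loops over the mesh's materials to append each indexed material name to that string.
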(event EventPrintObjectInfo
  (params (PrintScreen :type Boolean) (PrintLog :type Boolean))
  (bind _skeletalmeshcomponent (Variables|SkeletalMeshActor|GetSkeletalMeshComponent))
  (bind _skeletalmesh (Variables|/Script/Engine.SkinnedMeshComponent|GetSkeletalMesh _skeletalmeshcomponent))
  (bind _materials (Variables|/Script/Engine.SkeletalMesh|GetMaterials _skeletalmesh))
  (Development|PrintString (Utilities|String|Append "メッシュ名：" (Utilities|GetDisplayName _skeletalmesh) " 
マテリアル数：" (Utilities|String|ToString(Integer) (Utilities|Array|Length _materials)) " 
" (CallFunction|GetMaterialStr _materials) "骨の数：" (Utilities|String|ToString(Integer) (Class|SkinnedMeshComponent|GetNumBones _skeletalmeshcomponent))) PrintScreen PrintLog "(R=0.000000,G=0.660000,B=1.000000,A=1.000000)" 1e+01))

(fn ConstructionScript)

(fn GetMaterialStr
  (params (Materials :type Array%20of%20Skeletal%20Material%20Structures))
  (for (_array_element _array_index) Materials
    (LocalVariables|SetL_MatStr (Utilities|String|Append (LocalVariables|GetL_MatStr) (Utilities|String|Append "マテリアル名（" (Utilities|String|ToString(Integer) _array_index) "）：" (Utilities|GetDisplayName (Utilities|Struct|BreakSkeletalMaterial _array_element)) " 
"))))
  (return (LocalVariables|GetL_MatStr)))