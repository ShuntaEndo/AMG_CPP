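; Static mesh Blueprint that reports its own mesh and material information as Japanese-labeled debug text.
; The PrintObjectInfo event prints the mesh name and material count from its StaticMeshComponent, with flags selecting screen and log output.
; The GetMaterialStr helper loops over the component's materials to append each index and name to that message.
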(event EventPrintObjectInfo
  (params (PrintScreen :type Boolean) (PrintLog :type Boolean))
  (bind _staticmeshcomponent (Variables|Debug|GetStaticMeshComponent))
  (bind _returnvalue (Rendering|Material|GetMaterials _staticmeshcomponent))
  (Development|PrintString (Utilities|String|Append "メッシュ名：" (Utilities|GetDisplayName (Variables|/Script/Engine.StaticMeshComponent|GetStaticMesh _staticmeshcomponent)) " 
マテリアル数：" (Utilities|String|ToString(Integer) (Utilities|Array|Length _returnvalue)) " 
" (CallFunction|GetMaterialStr _returnvalue)) PrintScreen PrintLog "(R=0.000000,G=0.660000,B=1.000000,A=1.000000)" 1e+01))

(fn ConstructionScript)

(fn GetMaterialStr
  (params (Materials :type Array%20of%20Material%20Interface%20Object%20References))
  (for (_array_element _array_index) Materials
    (LocalVariables|SetL_MatStr (Utilities|String|Append (LocalVariables|GetL_MatStr) (Utilities|String|Append "マテリアル名（" (Utilities|String|ToString(Integer) _array_index) "）：" (Utilities|GetDisplayName _array_element) " 
"))))
  (return (LocalVariables|GetL_MatStr)))