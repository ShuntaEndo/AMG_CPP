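; BP_CubeRotator is an actor that spawns a grid of static mesh components and spins them continuously, resembling a component-count stress test.
; BeginPlay uses nested loops to add 500 evenly spaced meshes in a 50 by 10 layout at a raised relative height.
; Tick fetches every static mesh component by class each frame and adds a fixed world rotation, so spin speed depends on frame rate.
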(event EventBeginPlay
  (for _index (range 1 10) ; Y
    (for _index_2 (range 1 50) ; X
      (AddComponent|AddStaticMeshComponent false (Math|Transform|MakeTransform (Math|Vector|MakeVector (Math|Conversions|ToFloat(Integer) (* _index_2 200)) (Math|Conversions|ToFloat(Integer) (* _index 200)) 1e+03) "0, 0, 0" "1.000000,1.000000,1.000000")))))

(event EventTick
  (params (DeltaSeconds :type Float%20%28single-precision%29))
  (for _array_element (Actor|GetComponentsByClass "/Script/Engine.StaticMeshComponent")
    (Transformation|AddWorldRotation _array_element "0.000000,5.000000, 0" false false)))

(fn ConstructionScript)