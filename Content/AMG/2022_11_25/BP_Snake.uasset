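; BP_Snake is a spline Blueprint that builds a snake-like row of static meshes, with no active runtime logic.
; Its construction script walks the spline at a fixed Distance step, adding a mesh at each world-space point, sized by Scale divided by 100.
; Meshes use manual attachment, and the Spline itself is re-attached to each new mesh with keep-world rules, rather than the mesh to the Spline.
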(event EventBeginPlay)

(event Collision|EventActorBeginOverlap
  (params (OtherActor :type Actor%20Object%20Reference)))

(event EventTick
  (params (DeltaSeconds :type Float%20%28single-precision%29)))

(fn ConstructionScript
  (bind _spline (Variables|Default|GetSpline))
  (LocalVariables|SetL_Distance 0.0)
  (while (>= (Spline|GetDistanceAlongSplineatSplinePoint _spline (- (Spline|GetNumberOfSplinePoints _spline) 1)) (LocalVariables|GetL_Distance))
    (bind _returnvalue (AddComponent|AddStaticMeshComponent true (Math|Transform|MakeTransform (Spline|GetLocationatDistanceAlongSpline (Variables|Default|GetSpline) (LocalVariables|GetL_Distance) "World") "0, 0, 0" (Math|Conversions|ToVector(Float) (/ (Variables|Default|GetScale) 1e+02)))))
    (Transformation|AttachComponentToComponent (Variables|Default|GetSpline) _returnvalue "None" "KeepWorld" "KeepWorld" "KeepWorld" true)
    (LocalVariables|SetL_Distance (+ (LocalVariables|GetL_Distance) (Variables|Default|GetDistance)))))