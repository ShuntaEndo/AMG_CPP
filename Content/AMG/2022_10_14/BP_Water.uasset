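; BP_Water is a water volume that detects when the player camera is inside its Box component.
; Each tick it tests the camera location against the box's world location and scaled extent, ignoring box rotation.
; The result steps the Enable scalar in the MPC_Water parameter collection up or down, clamped between zero and one.
; This produces a short, frame-rate-dependent fade for any material reading that parameter.
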(event EventTick
  (params (DeltaSeconds :type Float%20%28single-precision%29))
  (bind _box (Variables|Default|GetBox))
  (bind _returnvalue (Rendering|Material|GetScalarParameterValue "/Game/AMG/2022_10_14/MPC_Water.MPC_Water" "Enable" :!class /Script/Engine.KismetMaterialLibrary))
  (Rendering|Material|SetScalarParameterValue "/Game/AMG/2022_10_14/MPC_Water.MPC_Water" "Enable" (Math|Float|Clamp(Float) (+ _returnvalue (* 0.1 (Math|Integer|SelectInt 1 -1 (Math|Geometry|IsPointinBox (Camera|GetCameraLocation (Game|GetPlayerCameraManager 0)) (Transformation|GetWorldLocation _box) (Components|Box|GetScaledBoxExtent _box)))))) :!class /Script/Engine.KismetMaterialLibrary))

(fn ConstructionScript)